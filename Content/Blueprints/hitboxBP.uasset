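; Fighting game hitbox actor that damages the opposing player and plays a punch sound.
; On hitboxSpawn it sets a display material by type (Proximity, Strike or Hurtbox), moves to HitboxLocation, hides the display and checks collision once.
; It compares its owner to the game mode's Player1 to pick the opponent, then passes damage, hitstun and blockstun if overlapping that player's Hurtbox.
; The collision check runs for every hitbox type.
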(event `hitboxSpawn`
  (switch `hitboxEnum` (`self.hitboxType`)
    (:`proximity_HB`
      (`PrimitiveComponent.SetMaterial` (`self.hitboxDisplay`) 0 "/Game/Materials/proximity.proximity"))
    (:`strike_HB`
      (`PrimitiveComponent.SetMaterial` (`self.hitboxDisplay`) 0 "/Game/Materials/strike.strike"))
    (:`hurtbox`
      (`PrimitiveComponent.SetMaterial` (`self.hitboxDisplay`) 0 "/Game/Materials/hurtbox.hurtbox")))
  (`SceneComponent.K2_SetWorldLocation` (`self.hitboxDisplay`) (`self.hitboxLocation`) false false)
  (`SceneComponent.SetVisibility` (`self.hitboxDisplay`) false false)
  (`self.CheckCollision`))

(event `CheckCollision`
  (bind _player1 (`FGGameMode.player1` (`self.FGGameMode`)))
  (bind _player2 (`FGGameMode.player2` (`self.FGGameMode`)))
  (bind _isplayer1 (`self.Determine Player`))
  (if _isplayer1
    (if (`self.IsOverlappingActor` (`FGCharacter.hurtbox` _player1))
      (`FGCharacter.takeDamage` _player1 (`self.hitboxDamage`) (`self.hitstunTime`) (`self.blockstunTime`))
      (`GameplayStatics.PlaySoundAtLocation` "/Game/Sound/mixkit-body-punch-quick-hit-2153.mixkit-body-punch-quick-hit-2153" (`self.K2_GetActorLocation` _player1) (struct) 1.0 1.0 0.0 null null null null))
    (elif (`self.IsOverlappingActor` (`FGCharacter.hurtbox` _player2))
      (`FGCharacter.takeDamage` _player2 (`self.hitboxDamage`) (`self.hitstunTime`) (`self.blockstunTime`))
      (`GameplayStatics.PlaySoundAtLocation` "/Game/Sound/mixkit-cartoon-punch-2149.mixkit-cartoon-punch-2149" (`self.K2_GetActorLocation` _player2) (struct) 1.0 1.0 0.0 null null null null))))

(fn `Determine Player`
  (returns (IsPlayer1 :type Boolean))
  (bind _asfggame_mode (cast `FGGameMode` (`GameplayStatics.GetGameMode`)))
  (bind _output_get (set `self.FGGameMode` _asfggame_mode))
  (if (== (`FGGameMode.player1` _output_get) (`self.GetOwner`))
    (return false)
    (else
      (return true))))

(fn `UserConstructionScript`)