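; Base NPC Blueprint that carries a hurtbox and chases the player character when in range.
; On BeginPlay it spawns a HurtBox at its own pawn transform, snaps it onto itself and becomes its owner.
; Each tick, while InRange is set and Distance exceeds a small threshold, it sets InputType to MoveRight and issues a simple move-to toward the player.
; InRange and Distance are only read in this graph.
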(event `self.ReceiveBeginPlay`
  (bind _output_get (set `self.playerTransform` (`self.GetTransform` (`PawnMovementComponent.GetPawnOwner` (`self.CharacterMovement`)))))
  (bind _returnvalue (`|SpawnActorFromClass` "/Game/Blueprints/hurtBox.hurtBox_C" _output_get "Undefined" "OverrideRootScale" null null))
  (bind _output_get_2 (set `self.hurtbox` _returnvalue))
  (`self.K2_AttachToActor` _output_get_2 self "None" "SnapToTarget" "SnapToTarget" "SnapToTarget" true)
  (`self.SetOwner` _returnvalue self))

(event `self.ReceiveTick`
  (params (DeltaSeconds :type "Float (single-precision)"))
  (if (`self.inRange`)
    (if (> (`self.distance`) 50.0)
      (set `self.inputType` "MoveRight")
      (`AIBlueprintHelperLibrary.SimpleMoveToActor` (`self.GetController`) (`GameplayStatics.GetPlayerCharacter` 0)))))

(fn `UserConstructionScript`)