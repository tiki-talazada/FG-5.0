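; Fighting game mode that spawns both fighters at match start and ends the match when Player 2's health runs out.
; Tagged PlayerStarts spawn classes chosen in BaseGameInstance: a possessed Player 1 and an NPC-variant Player 2, cross-linked before the HUB widget appears.
; Tick watches only Player 2's health, then shows EndRound and loads MatchEnd.
; The Alex choice returns no pawn for Player 1 and spawns NPC_BigBoss for Player 2.
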(event `self.ReceiveBeginPlay`
  (bind _player1 (`self.player1`))
  (bind _player2 (`self.player2`))
  (bind _outactors (`GameplayStatics.GetAllActorsOfClass` "/Script/Engine.PlayerStart"))
  (for _array_element _outactors
    (`self.SpawnPlayer` _array_element))
  (if (`KismetSystemLibrary.IsValid` (`self.player1`))
    (if (`KismetSystemLibrary.IsValid` (`self.player2`))
      (set `FGCharacter.otherPlayer` _player2 _player1)
      (set `FGCharacter.otherPlayer` _player1 _player2)
      (set `FGCharacter.facing` true _player2)
      (bind _returnvalue (`|CreateWidget` "/Game/Widgets/HUB.HUB_C" (`GameplayStatics.GetPlayerController` 0)))
      (`UserWidget.AddToViewport` _returnvalue 0))))

(event `self.ReceiveTick`
  (params (DeltaSeconds :type "Float (single-precision)"))
  (bind _player2 (`self.player2`))
  (`/Engine/EditorBlueprintResources/StandardMacros.IsValid` _player2
    (:`Is Valid`
      (if (<= (`FGCharacter.playerHealth` _player2) 0.0)
        (bind _returnvalue (`GameplayStatics.GetCurrentLevelName` true))
        (if (`KismetStringLibrary.NotEqual_StrStr` _returnvalue "MainScreen")
          (if (`KismetStringLibrary.NotEqual_StrStr` _returnvalue "CharacterSelect")
            (bind _returnvalue_2 (`|CreateWidget` "/Game/Widgets/EndRound.EndRound_C"))
            (`UserWidget.AddToViewport` _returnvalue_2 0)
            (`KismetSystemLibrary.Delay` 1.0)
            (`GameplayStatics.OpenLevel` "MatchEnd")))))))

(fn `DetermineCharClass`
  (params (spawnTransform :type "Transform Structure") (Actor :type "Actor Object Reference") (PlayerIndex :type Integer))
  (returns (CharacterReferences :type "FGCharacter Object Reference"))
  (bind _asbase_game_instance (cast `BaseGameInstance` (`GameplayStatics.GetGameInstance`)))
  (switch `int` PlayerIndex
    (:`0`
      (switch `CharClass` (`BaseGameInstance.P1characterClass` _asbase_game_instance)
        (:`Boss`
          (bind _returnvalue (`|SpawnActorFromClass` "/Game/Blueprints/CharacterBP/Boss/BossBP.BossBP_C" spawnTransform "Undefined" "OverrideRootScale" Actor null))
          (return _returnvalue))
        (:`Pink`
          (bind _returnvalue_2 (`|SpawnActorFromClass` "/Game/Blueprints/CharacterBP/Pink/PinkMannequinBP.PinkMannequinBP_C" spawnTransform "Undefined" "OverrideRootScale" Actor null))
          (return _returnvalue_2))
        (:`Alex`
          (`|SpawnActorFromClass` "/Game/Blueprints/CharacterBP/Alex.Alex_C" spawnTransform "Undefined" "OverrideRootScale" Actor null)
          (return null))))
    (:`1`
      (switch `CharClass` (`BaseGameInstance.P2characterClass` _asbase_game_instance)
        (:`Boss`
          (bind _returnvalue_3 (`|SpawnActorFromClass` "/Game/Blueprints/AI_Blueprint/Boss/NPC_BigBoss.NPC_BigBoss_C" spawnTransform "Undefined" "OverrideRootScale" Actor null))
          (return _returnvalue_3))
        (:`Pink`
          (bind _returnvalue_4 (`|SpawnActorFromClass` "/Game/Blueprints/AI_Blueprint/NPC_BP.NPC_BP_C" spawnTransform "Undefined" "OverrideRootScale" Actor null))
          (return _returnvalue_4))
        (:`Alex`
          (bind _returnvalue_5 (`|SpawnActorFromClass` "/Game/Blueprints/AI_Blueprint/Boss/NPC_BigBoss.NPC_BigBoss_C" spawnTransform "Undefined" "OverrideRootScale" Actor null))
          (return _returnvalue_5))))))

(fn `SpawnPlayer`
  (params (Object :type "Actor Object Reference"))
  (bind _asplayer_start (cast `PlayerStart` Object))
  (bind _playerstarttag (`PlayerStart.PlayerStartTag` _asplayer_start))
  (if (== "P1" _playerstarttag)
    ;[1 1 1] Possess
    (bind _characterreferences (`self.DetermineCharClass` (`self.GetTransform` Object) Object))
    (set `self.player1` _characterreferences)
    (`Controller.Possess` (`GameplayStatics.GetPlayerController` 0) _characterreferences)
    (elif (== _playerstarttag "P2")
      (bind _characterreferences_2 (`self.DetermineCharClass` (`self.GetTransform` Object) Object 1))
      (set `self.player2` _characterreferences_2))))

(fn `UserConstructionScript`)