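; DefaultCamera is a shared camera actor that keeps two players framed along the Y/Z plane.
; Shortly after BeginPlay it caches both player references from FGGameModeBP.
; Each tick it holds its X, centers Y between the players and sets Z from their summed heights with a slightly raised bias.
; Field of view scales with their horizontal separation, clamped to a fixed range, to zoom in and out.
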(event `self.ReceiveBeginPlay`
  (`KismetSystemLibrary.Delay` 0.03)
  (bind _asfggame_mode_bp (cast `/Game/Blueprints/FGGameModeBP` (`GameplayStatics.GetGameMode`)))
  (bind _player1 (`FGGameMode.player1` _asfggame_mode_bp))
  (`/Engine/EditorBlueprintResources/StandardMacros.IsValid` _player1
    (:`Is Valid`
      (set `self.Player1Refer` _player1)
      (bind _player2 (`FGGameMode.player2` _asfggame_mode_bp))
      (`/Engine/EditorBlueprintResources/StandardMacros.IsValid` _player2
        (:`Is Valid`
          (set `self.Player2Refer` _player2))))))

(event `self.ReceiveTick`
  (params (DeltaSeconds :type "Float (single-precision)"))
  (bind _player1refer (`self.Player1Refer`))
  (bind _player2refer (`self.Player2Refer`))
  (if (and (`KismetSystemLibrary.IsValid` _player1refer) (`KismetSystemLibrary.IsValid` _player2refer))
    (`self.K2_SetActorLocation` (`KismetMathLibrary.MakeVector` (.x (`self.K2_GetActorLocation`)) (/ (+ (.y (`self.K2_GetActorLocation` _player1refer)) (.y (`self.K2_GetActorLocation` _player2refer))) 2.0) (/ (+ (.z (`self.K2_GetActorLocation` _player1refer)) (.z (`self.K2_GetActorLocation` _player2refer))) 1.7)))
    (`CameraComponent.SetFieldOfView` (`self.CameraComponent`) (`KismetMathLibrary.FClamp` (`KismetMathLibrary.Abs` (* (- (.y (`self.K2_GetActorLocation` (`self.Player1Refer`))) (.y (`self.K2_GetActorLocation` (`self.Player2Refer`)))) 0.1)) 60.0 100.0))))

(fn `UserConstructionScript`)