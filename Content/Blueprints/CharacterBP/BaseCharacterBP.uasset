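; BaseCharacterBP is a base character Blueprint that gives the character a hurtbox and handles pausing the game.
; On BeginPlay it spawns a HurtBox actor at the pawn's transform, snaps it onto itself and sets itself as the owner.
; Pressing P pauses the game, adds a Pause widget to the viewport and shows the mouse cursor.
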(event `self.ReceiveBeginPlay`
  (bind _returnvalue (`|SpawnActorFromClass` "/Game/Blueprints/hurtBox.hurtBox_C" (`self.GetTransform` (`PawnMovementComponent.GetPawnOwner` (`self.CharacterMovement`))) "Undefined" "OverrideRootScale" null null))
  (bind _output_get (set `self.hurtbox` _returnvalue))
  (`self.K2_AttachToActor` _output_get self "None" "SnapToTarget" "SnapToTarget" "SnapToTarget" true)
  (`self.SetOwner` _returnvalue self))

(event `Key|P`
  (params (Key :type "Key Structure"))
  (:`Pressed`
    (`GameplayStatics.SetGamePaused` true)
    (bind _returnvalue (`|CreateWidget` "/Game/Widgets/Pause.Pause_C"))
    (`UserWidget.AddToViewport` _returnvalue 0)
    (set `PlayerController.bShowMouseCursor` true (`GameplayStatics.GetPlayerController` 0))))

(fn `UserConstructionScript`)